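; BP_Switch is an interactable switch with a text label and a colored button, which responds while something overlaps its box.
; Overlap start enables player 0 input, shows a press prompt and tints the button blue; overlap end disables input and restores the idle text and default color.
; E or gamepad top face button calls SwitchEvent, an empty hook here.
; The construction script creates the dynamic material and caches its default color.
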(event `self.Box.OnComponentBeginOverlap`
  (params (OverlappedComponent :type "PrimitiveComponent Object Reference") (OtherActor :type "Actor Object Reference") (OtherComp :type "PrimitiveComponent Object Reference") (OtherBodyIndex :type Integer) (bFromSweep :type Boolean) (SweepResult :type "HitResult Structure (by ref)"))
  (`self.EnableInput` (`GameplayStatics.GetPlayerController` 0))
  (bind _output_get (set `self.Text` "Press E"))
  (`TextRenderComponent.K2_SetText` (`self.TextRender`) _output_get)
  (`MaterialInstanceDynamic.SetVectorParameterValue` (`self.BoxMaterial`) "SwitchColor" (struct :`G` 0.085002 :`B` 0.93 :`A` 1.0)))

(event `self.Box.OnComponentEndOverlap`
  (params (OverlappedComponent :type "PrimitiveComponent Object Reference") (OtherActor :type "Actor Object Reference") (OtherComp :type "PrimitiveComponent Object Reference") (OtherBodyIndex :type Integer))
  (`self.DisableInput` (`GameplayStatics.GetPlayerController` 0))
  (bind _output_get (set `self.Text` "Stand"))
  (`TextRenderComponent.K2_SetText` (`self.TextRender`) _output_get)
  (`MaterialInstanceDynamic.SetVectorParameterValue` (`self.BoxMaterial`) "SwitchColor" (`self.DefaultColor`)))

(event `Key|E`
  (params (Key :type "Key Structure"))
  (:`Pressed`
    (`self.SwitchEvent` :!label _label)))

(event `SwitchEvent`)

(event `Key|Gamepad_FaceButton_Top`
  (params (Key :type "Key Structure"))
  (:`Pressed`
    (goto _label)))

(fn `UserConstructionScript`
  (`TextRenderComponent.K2_SetText` (`self.TextRender`) (`self.Text`))
  (bind _returnvalue (`PrimitiveComponent.CreateDynamicMaterialInstance` (`self.Button`) 0 null "None"))
  (bind _output_get (set `self.BoxMaterial` _returnvalue))
  (bind _returnvalue_2 (`MaterialInstanceDynamic.K2_GetVectorParameterValue` _output_get "SwitchColor"))
  (set `self.DefaultColor` _returnvalue_2))