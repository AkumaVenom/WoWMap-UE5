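; Switch Blueprint that randomizes the colors of a referenced water actor when triggered.
; On SwitchEvent it assigns new random RGB values to the water's overall, two Fresnel and fade colors.
; It then calls UpdateSettingsParameters on the water to apply them.
; The construction script only runs the parent's, and the other default events are unused.
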(event `SwitchEvent`
  (bind _waterreference (`self.WaterReference`))
  (bind _returnvalue (`KismetMathLibrary.MakeColor` (`KismetMathLibrary.RandomFloatInRange` 0.0 1.0) (`KismetMathLibrary.RandomFloatInRange` 0.0 1.0) (`KismetMathLibrary.RandomFloatInRange` 0.0 1.0)))
  (set `/Game/ISW5/Blueprint/BP_Water.Overall Color` _returnvalue _waterreference)
  (set `/Game/ISW5/Blueprint/BP_Water.FresnelColor1` _returnvalue _waterreference)
  (set `/Game/ISW5/Blueprint/BP_Water.FresnelColor2` _returnvalue _waterreference)
  (set `/Game/ISW5/Blueprint/BP_Water.FadeColor` _returnvalue _waterreference)
  (`/Game/ISW5/Blueprint/BP_Water.UpdateSettingsParameters` (`self.WaterReference`)))

(fn `UserConstructionScript`
  (`parent.UserConstructionScript`))